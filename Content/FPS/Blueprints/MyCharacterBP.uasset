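; First-person character Blueprint whose Fire and Fire2 inputs both toggle a Firing flag on press and release.
; StarFire and StopFire are empty stubs, with their bodies and calls left disconnected.
; The unwired shot logic runs randomly spread camera multi-line traces, lowering damage through Pared walls by their absorption value and printing it on enemy hits, using a HittedObjects list meant to skip repeats.
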(event `InputAction|Fire2` :overrideparent false
  (params (Key :type "Key Structure"))
  (:`Pressed`
    (set `self.Firing` true))
  (:`Released`
    (set `self.Firing` false)))

(event `InputAction|Fire` :overrideparent false
  (params (Key :type "Key Structure"))
  (:`Pressed`
    (set `self.Firing` true))
  (:`Released`
    (set `self.Firing` false)))

(fn `StarFire`
  (params (Amount :type Integer) (Shake :type "Float (double-precision)")))

(fn `StopFire`)

(fn `UserConstructionScript`)